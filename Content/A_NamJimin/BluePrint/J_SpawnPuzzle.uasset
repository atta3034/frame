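; J_SpawnPuzzle is a Blueprint that spawns the pieces of a grabbable jigsaw puzzle at BeginPlay.
; For each piece, it creates a J_PuzzlePiece widget with the image, piece count and grid coordinate derived from the loop index and the count's square root.
; It also spawns a J_GrabbablePuzzle at a random spot near the world origin at zero height, without passing it the widget.
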(event `self.ReceiveBeginPlay`
  (bind _returnvalue (`KismetMathLibrary.FTrunc` (`KismetMathLibrary.Sqrt` (`KismetMathLibrary.Conv_IntToDouble` (`self.NumberOfPieces`)))))
  (for _index (range 1 (+ (`self.NumberOfPieces`) 1))
    (`|CreateWidget` "/Game/A_NamJimin/BluePrint/J_PuzzlePiece.J_PuzzlePiece_C" null (`self.NumberOfPieces`) (`KismetMathLibrary.MakeVector2D` (`KismetMathLibrary.Conv_IntToDouble` (mod _index _returnvalue)) (`KismetMathLibrary.Conv_IntToDouble` (/ _index _returnvalue))) (`self.JigsawImage`))
    (`|SpawnActorFromClass` "/Game/A_NamJimin/BluePrint/J_GrabbablePuzzle.J_GrabbablePuzzle_C" (`KismetMathLibrary.Conv_VectorToTransform` (`KismetMathLibrary.MakeVector` (`KismetMathLibrary.RandomFloatInRange` -10.0 -100.0) (`KismetMathLibrary.RandomFloatInRange` -50.0 50.0))) "AdjustIfPossibleButAlwaysSpawn" "OverrideRootScale" null (0.0 0.0) 16 null)))

(fn `UserConstructionScript`)