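; J_KeyPadDoor is a keypad-locked door that unlocks when the correct code is entered.
; On BeginPlay it gets the J_KeyPad widget from its widget component and binds to its code-entered event.
; CheckCode clears the entry and unlocks on a match.
; While unlocked, Tick calls open/close every frame, with a FlipFlop alternating a timeline between forward and reverse to yaw the pivot.
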(event `Open/CloseDoor`
  (`/Engine/EditorBlueprintResources/StandardMacros.FlipFlop`
    (:`A`
      (bind (_direction _door_open) (`Timeline|타임라인` :!via `PlayFromStart` :!label _label)
        (:`Update`
          (`SceneComponent.K2_SetRelativeRotation` (`self.Pivot`) (`KismetMathLibrary.MakeRotator` 0.0 0.0 _door_open) false false))))
    (:`B`
      (goto _label :!via `ReverseFromEnd`))))

(event `self.ReceiveBeginPlay`
  (bind _asj_key_pad (cast `/Game/A_NamJimin/BluePrint/J_KeyPad` (`WidgetComponent.GetUserWidgetObject` (`self.KeyPadWidget`))))
  (bind _output_get (set `self.As J Key Pad` _asj_key_pad))
  (add `/Game/A_NamJimin/BluePrint/J_KeyPad.CodeEntered` _output_get (`|CreateDelegate` :!event `CheckCode`)))

(event `self.ReceiveTick`
  (params (DeltaSeconds :type "Float (single-precision)"))
  (if (not (`self.IsLocked`))
    (`self.Open/CloseDoor`)))

(fn `CheckCode`
  (params (CodeEntered :type String) (KeyPad :type "/Game/A_NamJimin/BluePrint/J_KeyPad Object Reference"))
  (if (`KismetStringLibrary.EqualEqual_StrStr` CodeEntered (`self.CorrectCode`))
    (set `self.IsLocked` false)
    (set `/Game/A_NamJimin/BluePrint/J_KeyPad.CurrentCode` "" (`self.As J Key Pad`))
    (else
      (set `/Game/A_NamJimin/BluePrint/J_KeyPad.CurrentCode` "" (`self.As J Key Pad`)))))

(fn `UserConstructionScript`)