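; Puzzle factory actor that spawns a set of J_GrabbablePuzzle pieces at its own transform on BeginPlay.
; A loop over NumberOfPieces turns each index into a 2D PuzzleCoordinate, using the truncated square root of the count as the grid width.
; Each piece receives that coordinate plus its loop index, passed through the piece's NumberOfPieces parameter.
; Spawning adjusts for collisions but always succeeds.
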(event `self.ReceiveBeginPlay`
  (bind _returnvalue (`KismetMathLibrary.FTrunc` (`KismetMathLibrary.Sqrt` (`KismetMathLibrary.Conv_IntToDouble` (`self.Number Of Pieces`)))))
  (for _index (range (`self.Number Of Pieces`))
    (`|SpawnActorFromClass` "/Game/A_NamJimin/BluePrint/J_GrabbablePuzzle.J_GrabbablePuzzle_C" (`self.GetTransform`) "AdjustIfPossibleButAlwaysSpawn" "OverrideRootScale" null (`KismetMathLibrary.MakeVector2D` (`KismetMathLibrary.Conv_IntToDouble` (mod _index _returnvalue)) (`KismetMathLibrary.Conv_IntToDouble` (/ _index _returnvalue))) _index null)))

(fn `UserConstructionScript`)