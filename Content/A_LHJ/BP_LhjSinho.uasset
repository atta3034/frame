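; Pedestrian traffic light Blueprint that cycles endlessly from BeginPlay through red, green and a blinking-green countdown.
; StartTrafficLight resets all lights, times each phase with Delays, then enters a once-per-second count loop that restarts the cycle at zero.
; Setter events toggle point lights and swap emissive materials.
; SetCounter splits the number into two LED digits through a "Number" material parameter, blanking the tens below 10.
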(event `self.ReceiveBeginPlay`
  (`self.Start Traffic Light`) ; 총괄함수를 호출하고
)

(event `Count Loop`
  ;[1 1 1] Comment
  ;;[0 0 0 1 12] 카운터 이벤트 진입
  (bind _result (`/Engine/EditorBlueprintResources/StandardMacros.DecrementInt` (`self.Current Count`) :!label _label)
    (:`  `
      ;;[0 0 0 1 12] 카운터 반복 조건
      (if (> _result 0)
        (`self.Set Counter` true (`self.Current Count`))
        (`self.Set Green Light` true)
        (`KismetSystemLibrary.Delay` 0.5)
        (`self.Set Green Light` false)
        (`KismetSystemLibrary.Delay` 0.5)
        (goto _label)
        (else
          ;;[0 0 0 1 12] 카운터 반복 탈출
          (`self.Start Traffic Light`))))))

(event `Start Traffic Light`
  ;[1 1 1] 신호등 순서
  (`self.Initialize`) ; 1.초기화시켠다
  (`self.Set Red Light` true) ; 2. 빨간불 함수를호출해서 켜준다(참으로 체크)
  (`KismetSystemLibrary.Delay` (`self.Red Light Duration`))
  (`self.Set Red Light` false) ; 끈다
  (`self.Set Green Light` true) ; 그린함수 호출
  (`KismetSystemLibrary.Delay` (`self.Green Light Duration`))
  ;[1 1 1] Comment
  (set `self.Current Count` (+ (`self.Count`) 1)) ; 현재카운트에 1씩 증가해준다
  (goto _label))

(event `INITIALIZE_TEST`
  ;[1 1 1] <참고> 커스텀 함수를 만들고 그 함수를 호출하고
)

(event `CustomEvent`
  ;[1 1 1] <참고> 커스텀 함수를 만들고 그 함수를 호출하고
)

(event `light loop`
  ;[1 1 1] <참고>  차이
)

(event `Initialize`
  ;[1 1 1] 초기화. 모든 불을 끈다.
  (`self.Set Red Light` false) ; 빨간불 함수에서 불린값을 OFF 로
  (`self.Set Green Light` false) ; 초록불 함수
  (`self.Set Counter` false) ; 숫자관련 함수
)

(event `Set Red Light`
  (params (On :type Boolean))
  ;[1 0.2191 0.7935] 빨간불 On / Off 하는 이벤트- 머티리얼을 교체함으로 해서
  (`SceneComponent.SetVisibility` (`self.PointLight_RedMark`) On false) ; 빨간조명 보이게 한다
  (`PrimitiveComponent.SetMaterial` (`self.TL_Human_3wayMirror_RedLight_EM`) 0 (select `bool` On :`false` "/Game/01_Assets/09_TrafficLight/신호등/material/Light/M_Emissive_Off.M_Emissive_Off" :`true` "/Game/01_Assets/09_TrafficLight/신호등/material/Light/MI_Emissive_Red.MI_Emissive_Red" :!type "MaterialInterface Object Reference")) ; 머티리얼을 교체한다
)

(event `Set Green Light`
  (params (On :type Boolean))
  ;[1 1 1] 초록불 On / Off 하는 이벤트
  (`SceneComponent.SetVisibility` (`self.PointLight_GreenMark`) On false) ; 그린조명 보이게 한다
  (`PrimitiveComponent.SetMaterial` (`self.TL_Human_3wayMirror_GreenLight_EM`) 0 (select `bool` On :`false` "/Game/01_Assets/09_TrafficLight/신호등/material/Light/M_Emissive_Off.M_Emissive_Off" :`true` "/Game/01_Assets/09_TrafficLight/신호등/material/Light/MI_Emissive_Green.MI_Emissive_Green" :!type "MaterialInterface Object Reference")) ; 머티리얼을 교체한다
)

(event `Set Counter`
  (params (On :type Boolean) (Number :type Integer))
  ;[1 1 1] 숫자 On / Off 그리고 숫자 설정해주는 이벤트
  (`SceneComponent.SetVisibility` (`self.PointLight_Counter`) On false)
  (`PrimitiveComponent.SetMaterial` (`self.TL_Human_CounterLED_Mesh`) 0 (select `bool` On :`false` "/Game/01_Assets/09_TrafficLight/신호등/material/Light/M_Emissive_Num_Off.M_Emissive_Num_Off" :`true` "/Game/01_Assets/09_TrafficLight/신호등/material/Light/M_Emissive_Num_On.M_Emissive_Num_On" :!type "MaterialInterface Object Reference"))
  (`PrimitiveComponent.SetMaterial` (`self.TL_Human_CounterLED_Mesh1`) 0 (select `bool` On :`false` "/Game/01_Assets/09_TrafficLight/신호등/material/Light/M_Emissive_Num_Off.M_Emissive_Num_Off" :`true` "/Game/01_Assets/09_TrafficLight/신호등/material/Light/M_Emissive_Num_On.M_Emissive_Num_On" :!type "MaterialInterface Object Reference")) ; 2개의 머티리얼을 셋
  ;[1 1 1] 불이 켜져있다면 숫자 설정
  (if On
    (`MeshComponent.SetScalarParameterValueOnMaterials` (`self.TL_Human_CounterLED_Mesh`) "Number" (`KismetMathLibrary.Conv_IntToDouble` (/ Number 10))) ; 10의자리 셋, 파라미터이름은 Number 는 머티리얼의 값이다
    (`MeshComponent.SetScalarParameterValueOnMaterials` (`self.TL_Human_CounterLED_Mesh1`) "Number" (`KismetMathLibrary.Conv_IntToDouble` (mod Number 10))) ; 1의자리 셋
    ;[1 1 1] 10 이하라면 10의자리 불 꺼주기
    (if (< Number 10)
      (`PrimitiveComponent.SetMaterial` (`self.TL_Human_CounterLED_Mesh`) 0 "/Game/01_Assets/09_TrafficLight/신호등/material/Light/M_Emissive_Num_Off.M_Emissive_Num_Off") ; 숫자가 꺼지는 머티리얼을 셋한다
    )))

(fn `UserConstructionScript`)